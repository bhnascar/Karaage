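; A Coherent UI HUD Blueprint that displays an HTML page (hud.html) as the game HUD.
; On BeginPlay it spawns and initializes an input actor that always accepts mouse input, then sets up the UI view.
; Once UI scripting is ready, it binds a JavaScript event handler that switches on event name.
; The switch and the key-down handler are empty stubs.
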(event `CoUIKeyDown_Event`
  (params (Key :type "CoherentUIInputActor.ECoherentUIKeys Enum" :default "LeftMouseButton")))

(event `self.ReceiveBeginPlay`
  (bind _returnvalue (`|SpawnActorFromClass` "/Script/CoherentUIPlugin.CoherentUIInputActor" (`KismetMathLibrary.MakeTransform` (0.0 0.0 0.0))))
  (`CoherentUIInputActor.Initialize` _returnvalue "ECC_WorldDynamic" "TA_Wrap" "RQ_Balanced" 0)
  (add `CoherentUIInputActor.OnCoherentInputActorKeyDown` _returnvalue (delegate `CoUIKeyDown_Event`))
  (`CoherentUIInputActor.AlwaysAcceptMouseInput` _returnvalue true)
  (add `CoherentBaseComponent.UIScriptingReady` (`self.CoherentUIHUD`) (delegate `UIScriptingReady_Event`))
  (`self.SetupUIView` self "coui://uiresources/hud.html" false true 0.0 true 30 false))

(event `UIScriptingReady_Event`
  (add `CoherentBaseComponent.JavaScriptEvent` (`self.CoherentUIHUD`) (delegate `JavaScriptEvent_Event_0`)))

(event `JavaScriptEvent_Event_0`
  (params (payload :type "CoherentUIJSPayload Object Reference"))
  (switch `string` (`CoherentUIJSPayload.EventName` payload)))

(fn `UserConstructionScript`)